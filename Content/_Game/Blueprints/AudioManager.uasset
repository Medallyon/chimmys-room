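; AudioManager plays 2D background audio when play begins, if its Enabled flag is set.
; With a valid CueBGStart, it plays that intro, waits out its duration plus a short gap, then starts CueBGMusic.
; Without an intro, a valid CueBGMusic triggers a low-volume SpawnSound2D call, though that call shows no sound input connected.
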(event `self.ReceiveBeginPlay`
  (if (`self.Enabled`)
    (`/Engine/EditorBlueprintResources/StandardMacros.IsValid` (`self.Cue_BGStart`)
      (:`Is Valid`
        (`GameplayStatics.SpawnSound2D` (`self.Cue_BGStart`) 1.0 1.0 0.0 null false false)
        (`KismetSystemLibrary.Delay` (+ (`SoundBase.Duration` (`self.Cue_BGStart`)) 0.33))
        (`GameplayStatics.SpawnSound2D` (`self.Cue_BGMusic`) 1.0 1.0 0.0 null))
      (:`Is Not Valid`
        (`/Engine/EditorBlueprintResources/StandardMacros.IsValid` (`self.Cue_BGMusic`)
          (:`Is Valid`
            (`GameplayStatics.SpawnSound2D` null 0.1 1.0 0.0 null)))))))

(fn `UserConstructionScript`)