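; Customizable picture frame actor that builds its look in the Construction Script from a choice of four frame styles and a picture material.
; The ActiveFrame selection sets an index that picks the frame mesh and, halved minus one, an ImagePlanes child as the active image plane.
; ActivateSelectedFrame runs a destroy loop over ImagePlanes children after a RemoveIndex meant to spare that plane, which then receives PictureMaterial.
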(fn `UserConstructionScript`
  (`|ExecutionSequence`
    (:`then_0`
      (switch `/Game/_Game/Blueprints/CustomPaintingFrame/Enum_Frames` (`self.ActiveFrame`)
        (:`NewEnumerator0`
          (set `self.CurrentFrame` 0))
        (:`NewEnumerator1`
          (set `self.CurrentFrame` 1))
        (:`NewEnumerator2`
          (set `self.CurrentFrame` 2))
        (:`NewEnumerator3`
          (set `self.CurrentFrame` 3)))
      (`self.ActivateSelectedFrame`
        (:`Completed`
          (`StaticMeshComponent.SetStaticMesh` (`self.StaticMesh`) (`|GetArrayItem` (`self.SMs_Frames`) (`self.CurrentFrame`))))))
    (:`then_1`
      (bind _asprimitive_component (cast `PrimitiveComponent` (`self.ActiveImagePlane`)))
      (`PrimitiveComponent.SetMaterial` _asprimitive_component 0 (`self.PictureMaterial`)))))