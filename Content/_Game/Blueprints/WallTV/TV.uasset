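; Wall-mounted flat TV actor that opens a video source on its MediaPlayer at BeginPlay.
; The construction script sets the screen slot to ScreenMaterial if valid, otherwise creates a dynamic material instance and sets ScreenTexture on it, though the parameter name is None.
; It also assigns a separate light function material to each of three R, G and B spotlights.
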(event `self.ReceiveBeginPlay`
  (`MediaPlayer.OpenSource` (`self.MediaPlayer`) "/Game/Movies/video.video"))

(fn `UserConstructionScript`
  (`|ExecutionSequence`
    (:`then_0`
      ;[0 0.2969 1] Apply Material or Texture to the screen
      (`/Engine/EditorBlueprintResources/StandardMacros.IsValid` (`self.ScreenMaterial`)
        (:`Is Valid`
          (`PrimitiveComponent.SetMaterial` (`self.SM_Prop_Television_Flat_Wall_01`) 1 (`self.ScreenMaterial`)))
        (:`Is Not Valid`
          (bind _returnvalue (`PrimitiveComponent.CreateDynamicMaterialInstance` (`self.SM_Prop_Television_Flat_Wall_01`) 1 null "None"))
          (bind _output_get (set `self.TV_DynamicMaterial` _returnvalue))
          (`MaterialInstanceDynamic.SetTextureParameterValue` _returnvalue "None" (`self.ScreenTexture`))
          (`MaterialInstanceDynamic.SetTextureParameterValue` _output_get "None" (`self.ScreenTexture`)))))
    (:`then_1`
      ;[0 1 0.25] Apply LightFunctions to respective RGB Spotlights
      (`LightComponent.SetLightFunctionMaterial` (`self.R`) (`|GetArrayItem` (`self.LightFunctions`)))
      (`LightComponent.SetLightFunctionMaterial` (`self.G`) (`|GetArrayItem` (`self.LightFunctions`) 1))
      (`LightComponent.SetLightFunctionMaterial` (`self.B`) (`|GetArrayItem` (`self.LightFunctions`) 2)))))