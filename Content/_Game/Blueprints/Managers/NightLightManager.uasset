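; Sun light manager that drives day and night from its own rotation and switches a set of lights.
; Tick eases sun intensity by pitch during day; past a pitch threshold it fades the sun and enables the lights once via a resettable DoOnce.
; Returning to day clears NightTime without turning lights off.
; Enable, disable and toggle functions update NightTime, with enable and disable also firing notifications.
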(event `self.ReceiveTick`
  (params (DeltaSeconds :type "Float (single-precision)"))
  (bind (_returnvalue_roll _returnvalue_pitch) (`KismetMathLibrary.BreakRotator` (`self.K2_GetActorRotation`)))
  (bind _returnvalue (`KismetMathLibrary.NormalizeToRange` _returnvalue_pitch -90.0 90.0))
  (set `self.DeltaSeconds` DeltaSeconds)
  (`|ExecutionSequence`
    (:`then_0`
      (if (>= _returnvalue_pitch 30.0)
        (`|ExecutionSequence`
          (:`then_0`
            (`LightComponent.SetIntensity` (`self.SunLightComponent`) (`KismetMathLibrary.FInterpTo` (`LightComponentBase.Intensity` (`self.SunLightComponent`)) 0.0 (`self.DeltaSeconds`) 1.0)))
          (:`then_1`
            (`/Engine/EditorBlueprintResources/StandardMacros.DoOnce` false :!label _label
              (:`Completed`
                (`|ExecutionSequence`
                  (:`then_0`
                    (set `self.NightTime` true))
                  (:`then_1`
                    (`self.EnableLights`)))))))
        (else
          (set `self.NightTime` false)
          (goto _label :!via `Reset`))))
    (:`then_1`
      (if (not (`self.NightTime`))
        (`LightComponent.SetIntensity` (`self.SunLightComponent`) (`KismetMathLibrary.FInterpEaseInOut` 5.5 0.0 _returnvalue 10.0))
        (`LightComponent.SetIntensity` (`self.SunLightComponent`) (`KismetMathLibrary.FInterpEaseInOut` 50.0 0.0 _returnvalue 10.0))))))

(event `self.ReceiveBeginPlay`
  (set `self.SunLightComponent` (`Light.LightComponent`)))

(fn `DisableLights`
  (for _array_element (`self.Lights`)
    (`/Game/InteractiveLights/Blueprints/BaseElements/Light_Base.Turn Off` _array_element))
  (set `self.NightTime` false)
  (`self.DisabledLights`))

(fn `EnableLights`
  (for _array_element (`self.Lights`)
    (`/Game/InteractiveLights/Blueprints/BaseElements/Light_Base.Turn On` _array_element))
  (set `self.NightTime` true)
  (`self.EnabledLights`))

(fn `ToggleLights`
  (if (`self.NightTime`)
    (`self.DisableLights`)
    (else
      (`self.EnableLights`))))

(fn `UserConstructionScript`)