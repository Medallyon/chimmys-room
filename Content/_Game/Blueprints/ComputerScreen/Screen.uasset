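; Computer screen Blueprint that plays a random media file and pairs the screen with red, green and blue spotlights.
; The construction script applies ScreenMaterial to the Video component, or falls back to a dynamic material instance that is given ScreenTexture.
; It also assigns a separate light function material to each of the three spotlights.
; On BeginPlay, the MediaPlayer opens a random source from MediaFiles.
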(event `self.ReceiveBeginPlay`
  (bind _mediafiles (`self.MediaFiles`))
  (`MediaPlayer.OpenSource` (`self.MediaPlayer`) (`|GetArrayItem` _mediafiles (`KismetMathLibrary.RandomIntegerInRange` 0 (`KismetArrayLibrary.Array_LastIndex` _mediafiles)))))

(fn `UserConstructionScript`
  (`|ExecutionSequence`
    (:`then_0`
      ;[0 0.2969 1] Apply Material or Texture to the screen
      (`/Engine/EditorBlueprintResources/StandardMacros.IsValid` (`self.ScreenMaterial`)
        (:`Is Valid`
          (`PrimitiveComponent.SetMaterial` (`self.Video`) 0 (`self.ScreenMaterial`)))
        (:`Is Not Valid`
          (bind _returnvalue (`PrimitiveComponent.CreateDynamicMaterialInstance` (`self.Video`) 0 null "None"))
          (bind _output_get (set `self.TV_DynamicMaterial` _returnvalue))
          (`MaterialInstanceDynamic.SetTextureParameterValue` _returnvalue "None" (`self.ScreenTexture`))
          (`MaterialInstanceDynamic.SetTextureParameterValue` _output_get "None" (`self.ScreenTexture`)))))
    (:`then_1`
      ;[0 1 0.25] Apply LightFunctions to respective RGB Spotlights
      (`LightComponent.SetLightFunctionMaterial` (`self.R`) (`|GetArrayItem` (`self.LightFunctions`)))
      (`LightComponent.SetLightFunctionMaterial` (`self.G`) (`|GetArrayItem` (`self.LightFunctions`) 1))
      (`LightComponent.SetLightFunctionMaterial` (`self.B`) (`|GetArrayItem` (`self.LightFunctions`) 2)))))