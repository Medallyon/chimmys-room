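; Collectible pickup actor that spins its mesh every tick and is collected when a Chimmy overlaps its sphere collider.
; On overlap it reports itself to the DatabaseManager, found in the level at BeginPlay, then destroys itself.
; The construction script applies the configurable mesh and raises it by a vertical offset.
; Rotation is a fixed step per tick, not scaled by delta time.
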(event `self.ReceiveBeginPlay`
  (bind _outactors (`GameplayStatics.GetAllActorsOfClass` "/Game/_Game/Blueprints/DatabaseManager.DatabaseManager_C"))
  (set `self.DB` (`|GetArrayItem` _outactors)))

(event `self.ReceiveTick`
  (params (DeltaSeconds :type "Float (single-precision)"))
  (`|ExecutionSequence`
    (:`then_0`
      (`SceneComponent.K2_AddLocalRotation` (`self.StaticMesh`) (`KismetMathLibrary.MakeRotator` 0.0 0.0 (`self.RotationSpeed`)) false false))))

(event `self.SphereCollider.OnComponentBeginOverlap`
  (params (OverlappedComponent :type "PrimitiveComponent Object Reference") (OtherActor :type "Actor Object Reference") (OtherComp :type "PrimitiveComponent Object Reference") (OtherBodyIndex :type Integer) (bFromSweep :type Boolean) (SweepResult :type "HitResult Structure (by ref)"))
  (cast `/Game/_Game/Blueprints/Character/Chimmy` OtherActor)
  (`/Game/_Game/Blueprints/DatabaseManager.CollectibleActivated` (`self.DB`) self)
  (`self.K2_DestroyActor`))

(fn `UserConstructionScript`
  (`|ExecutionSequence`
    (:`then_0`
      (`self.Construction_SetStaticMesh`))
    (:`then_1`
      (`self.Construction_AddVerticalOffset`))))